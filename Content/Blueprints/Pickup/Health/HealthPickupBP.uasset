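; Health pickup actor that restores health to an FPSController entering its Trigger component.
; On overlap, it casts the other actor and compares current health to the maximum.
; Below maximum, it adds HealthPoints without clamping the result, then destroys itself.
; At or above maximum, it sets health to the maximum and stays in the level.
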(event OnComponentBeginOverlap(Trigger)
  (params (OverlappedComponent :type Primitive%20Component%20Object%20Reference) (OtherActor :type Actor%20Object%20Reference) (OtherComp :type Primitive%20Component%20Object%20Reference) (OtherBodyIndex :type Integer) (bFromSweep :type Boolean) (SweepResult :type Hit%20Result%20Structure%20%28by%20ref%29))
  (bind _asfpscontroller (Utilities|Casting|CastToFPSController OtherActor))
  (if (>= (Variables|/Game/Blueprints/PlayerBP/FPSController.FPSController_C|GetCurrentHealth _asfpscontroller) (Variables|/Game/Blueprints/PlayerBP/FPSController.FPSController_C|GetMaxHealth _asfpscontroller))
    (Variables|/Game/Blueprints/PlayerBP/FPSController.FPSController_C|SetCurrentHealth _asfpscontroller (Variables|/Game/Blueprints/PlayerBP/FPSController.FPSController_C|GetMaxHealth _asfpscontroller))
    (else
      (Variables|/Game/Blueprints/PlayerBP/FPSController.FPSController_C|SetCurrentHealth _asfpscontroller (+ (Variables|/Game/Blueprints/PlayerBP/FPSController.FPSController_C|GetCurrentHealth _asfpscontroller) (Variables|Default|GetHealthPoints)))
      (Actor|DestroyActor))))

(fn ConstructionScript)