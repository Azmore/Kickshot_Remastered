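; CrosshairHUD is a HUD Blueprint that draws a crosshair at the middle of the screen.
; On each DrawHUD event it halves the screen size, applies a fixed offset and draws the Crosshair texture as a small square.
; The tint and opacity come from the Red, Green, Blue and Alpha variables.
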(event EventDrawHUD
  (params (SizeX :type Integer) (SizeY :type Integer))
  (Canvas|DrawTexture "/Game/Art/Crosshairs/crosshair.crosshair" (Math|Conversions|ToFloat(Integer) (+ (/ SizeX 2) -7)) (Math|Conversions|ToFloat(Integer) (+ (/ SizeY 2) -7)) 16.0 16.0 0.0 0.0 1.0 1.0 (Utilities|Struct|MakeLinearColor (Variables|Default|GetRed) (Variables|Default|GetGreen) (Variables|Default|GetBlue) (Variables|Default|GetAlpha)) "BLEND_Translucent" 1.0 true))

(fn ConstructionScript)