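; Flying spotlight turret enemy that sweeps random points around its spawn, hunts the player and dies at zero health.
; Entering the construction-script-sized capsule trigger stops flight and starts clamped-pitch tracking; a line trace confirms sight before firing.
; A shooting timeline swaps the barrel material as a warning, then spawns a bullet when finished.
; On trigger exit, it flies near the player's last location while turning toward them, and resumes idle spinning.
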(event OnComponentBeginOverlap(Trigger)
  (params (OverlappedComponent :type Primitive%20Component%20Object%20Reference) (OtherActor :type Actor%20Object%20Reference) (OtherComp :type Primitive%20Component%20Object%20Reference) (OtherBodyIndex :type Integer) (bFromSweep :type Boolean) (SweepResult :type Hit%20Result%20Structure%20%28by%20ref%29))
  (bind _body (Variables|Default|GetBody))
  ;[1 1 1] Targetting Player
  (bind _asfpscontroller (Utilities|Casting|CastToFPSController OtherActor))
  (Variables|Default|SetFlyingEnabled? false)
  (CallFunction|StartTargetting)
  (CallFunction|StopIdleAnimation)
  (Variables|Default|SetPlayerInside? true)
  (Timeline|TargetPlayer Play
    (:Update
      (if (and (Utilities|IsValid _body) (Class|AIBlueprintHelperLibrary|IsValidAIRotation (Math|Rotator|MakeRotator (.Roll (Math|Rotator|BreakRotator (Class|KismetMathLibrary|RInterptoConstant (Transformation|GetWorldRotation (Variables|Default|GetBody)) (Math|Rotator|FindLookatRotation (Transformation|GetActorLocation) (- (Transformation|GetWorldLocation (Variables|/Game/Blueprints/PlayerBP/FPSController.FPSController_C|GetRootLocation _asfpscontroller)) (Math|Vector|MakeVector 0.0 0.0 1e+02))) 1.0 (Variables|TurretTargetting|GetTargetPlayerSpeed)))) (Math|Float|ClampAngle (.Pitch (Math|Rotator|BreakRotator (Class|KismetMathLibrary|RInterptoConstant (Transformation|GetWorldRotation (Variables|Default|GetBody)) (Math|Rotator|FindLookatRotation (Transformation|GetActorLocation) (- (Transformation|GetWorldLocation (Variables|/Game/Blueprints/PlayerBP/FPSController.FPSController_C|GetRootLocation _asfpscontroller)) (Math|Vector|MakeVector 0.0 0.0 1e+02))) 1.0 (Variables|TurretTargetting|GetTargetPlayerSpeed)))) (Variables|TurretTargetting|GetMinAngleRotationInDegrees) (Variables|TurretTargetting|GetMaxAngleRotationInDegrees)) (.Yaw (Math|Rotator|BreakRotator (Class|KismetMathLibrary|RInterptoConstant (Transformation|GetWorldRotation (Variables|Default|GetBody)) (Math|Rotator|FindLookatRotation (Transformation|GetActorLocation) (- (Transformation|GetWorldLocation (Variables|/Game/Blueprints/PlayerBP/FPSController.FPSController_C|GetRootLocation _asfpscontroller)) (Math|Vector|MakeVector 0.0 0.0 1e+02))) 1.0 (Variables|TurretTargetting|GetTargetPlayerSpeed)))))))
        (Transformation|SetWorldRotation _body (Math|Rotator|MakeRotator (.Roll (Math|Rotator|BreakRotator (Class|KismetMathLibrary|RInterptoConstant (Transformation|GetWorldRotation (Variables|Default|GetBody)) (Math|Rotator|FindLookatRotation (Transformation|GetActorLocation) (- (Transformation|GetWorldLocation (Variables|/Game/Blueprints/PlayerBP/FPSController.FPSController_C|GetRootLocation _asfpscontroller)) (Math|Vector|MakeVector 0.0 0.0 1e+02))) 1.0 (Variables|TurretTargetting|GetTargetPlayerSpeed)))) (Math|Float|ClampAngle (.Pitch (Math|Rotator|BreakRotator (Class|KismetMathLibrary|RInterptoConstant (Transformation|GetWorldRotation (Variables|Default|GetBody)) (Math|Rotator|FindLookatRotation (Transformation|GetActorLocation) (- (Transformation|GetWorldLocation (Variables|/Game/Blueprints/PlayerBP/FPSController.FPSController_C|GetRootLocation _asfpscontroller)) (Math|Vector|MakeVector 0.0 0.0 1e+02))) 1.0 (Variables|TurretTargetting|GetTargetPlayerSpeed)))) (Variables|TurretTargetting|GetMinAngleRotationInDegrees) (Variables|TurretTargetting|GetMaxAngleRotationInDegrees)) (.Yaw (Math|Rotator|BreakRotator (Class|KismetMathLibrary|RInterptoConstant (Transformation|GetWorldRotation (Variables|Default|GetBody)) (Math|Rotator|FindLookatRotation (Transformation|GetActorLocation) (- (Transformation|GetWorldLocation (Variables|/Game/Blueprints/PlayerBP/FPSController.FPSController_C|GetRootLocation _asfpscontroller)) (Math|Vector|MakeVector 0.0 0.0 1e+02))) 1.0 (Variables|TurretTargetting|GetTargetPlayerSpeed))))) false false)
        (Utilities|LineTrace
          (:End
            (if (and (Variables|Default|GetCanShoot?) (Variables|Default|GetTargetPlayer?))
              (Variables|Default|SetCanShoot? false)
              (CallFunction|StartShooting)
              (Variables|Default|SetTurretRechargeTimeStart (Variables|Default|GetTimeInSeconds)))))))))

(event OnComponentEndOverlap(Trigger)
  (params (OverlappedComponent :type Primitive%20Component%20Object%20Reference) (OtherActor :type Actor%20Object%20Reference) (OtherComp :type Primitive%20Component%20Object%20Reference) (OtherBodyIndex :type Integer))
  (bind _body (Variables|Default|GetBody))
  ;[1 1 1] Targetting Player
  (bind _asfpscontroller (Utilities|Casting|CastToFPSController OtherActor))
  (CallFunction|GotoPlayerLocation (Transformation|GetWorldLocation (Variables|/Script/Engine.Character|GetCapsuleComponent _asfpscontroller)))
  (CallFunction|StartSweep)
  (Variables|Default|SetFlyingEnabled? true)
  (Variables|Default|SetTargetPlayer? false)
  (CallFunction|IdleAnimation)
  (Variables|Default|SetPlayerInside? false)
  (Timeline|TargetPlayer Stop
    (:Update
      (if (and (Utilities|IsValid _body) (Class|AIBlueprintHelperLibrary|IsValidAIRotation (Math|Rotator|MakeRotator (.Roll (Math|Rotator|BreakRotator (Class|KismetMathLibrary|RInterptoConstant (Transformation|GetWorldRotation (Variables|Default|GetBody)) (Math|Rotator|FindLookatRotation (Transformation|GetActorLocation) (- (Transformation|GetWorldLocation (Variables|/Game/Blueprints/PlayerBP/FPSController.FPSController_C|GetRootLocation (stale OnComponentBeginOverlap(Trigger) _asfpscontroller))) (Math|Vector|MakeVector 0.0 0.0 1e+02))) 1.0 (Variables|TurretTargetting|GetTargetPlayerSpeed)))) (Math|Float|ClampAngle (.Pitch (Math|Rotator|BreakRotator (Class|KismetMathLibrary|RInterptoConstant (Transformation|GetWorldRotation (Variables|Default|GetBody)) (Math|Rotator|FindLookatRotation (Transformation|GetActorLocation) (- (Transformation|GetWorldLocation (Variables|/Game/Blueprints/PlayerBP/FPSController.FPSController_C|GetRootLocation (stale OnComponentBeginOverlap(Trigger) _asfpscontroller))) (Math|Vector|MakeVector 0.0 0.0 1e+02))) 1.0 (Variables|TurretTargetting|GetTargetPlayerSpeed)))) (Variables|TurretTargetting|GetMinAngleRotationInDegrees) (Variables|TurretTargetting|GetMaxAngleRotationInDegrees)) (.Yaw (Math|Rotator|BreakRotator (Class|KismetMathLibrary|RInterptoConstant (Transformation|GetWorldRotation (Variables|Default|GetBody)) (Math|Rotator|FindLookatRotation (Transformation|GetActorLocation) (- (Transformation|GetWorldLocation (Variables|/Game/Blueprints/PlayerBP/FPSController.FPSController_C|GetRootLocation (stale OnComponentBeginOverlap(Trigger) _asfpscontroller))) (Math|Vector|MakeVector 0.0 0.0 1e+02))) 1.0 (Variables|TurretTargetting|GetTargetPlayerSpeed)))))))
        (Transformation|SetWorldRotation _body (Math|Rotator|MakeRotator (.Roll (Math|Rotator|BreakRotator (Class|KismetMathLibrary|RInterptoConstant (Transformation|GetWorldRotation (Variables|Default|GetBody)) (Math|Rotator|FindLookatRotation (Transformation|GetActorLocation) (- (Transformation|GetWorldLocation (Variables|/Game/Blueprints/PlayerBP/FPSController.FPSController_C|GetRootLocation (stale OnComponentBeginOverlap(Trigger) _asfpscontroller))) (Math|Vector|MakeVector 0.0 0.0 1e+02))) 1.0 (Variables|TurretTargetting|GetTargetPlayerSpeed)))) (Math|Float|ClampAngle (.Pitch (Math|Rotator|BreakRotator (Class|KismetMathLibrary|RInterptoConstant (Transformation|GetWorldRotation (Variables|Default|GetBody)) (Math|Rotator|FindLookatRotation (Transformation|GetActorLocation) (- (Transformation|GetWorldLocation (Variables|/Game/Blueprints/PlayerBP/FPSController.FPSController_C|GetRootLocation (stale OnComponentBeginOverlap(Trigger) _asfpscontroller))) (Math|Vector|MakeVector 0.0 0.0 1e+02))) 1.0 (Variables|TurretTargetting|GetTargetPlayerSpeed)))) (Variables|TurretTargetting|GetMinAngleRotationInDegrees) (Variables|TurretTargetting|GetMaxAngleRotationInDegrees)) (.Yaw (Math|Rotator|BreakRotator (Class|KismetMathLibrary|RInterptoConstant (Transformation|GetWorldRotation (Variables|Default|GetBody)) (Math|Rotator|FindLookatRotation (Transformation|GetActorLocation) (- (Transformation|GetWorldLocation (Variables|/Game/Blueprints/PlayerBP/FPSController.FPSController_C|GetRootLocation (stale OnComponentBeginOverlap(Trigger) _asfpscontroller))) (Math|Vector|MakeVector 0.0 0.0 1e+02))) 1.0 (Variables|TurretTargetting|GetTargetPlayerSpeed))))) false false)
        (Utilities|LineTrace
          (:End
            (if (and (Variables|Default|GetCanShoot?) (Variables|Default|GetTargetPlayer?))
              (Variables|Default|SetCanShoot? false)
              (CallFunction|StartShooting)
              (Variables|Default|SetTurretRechargeTimeStart (Variables|Default|GetTimeInSeconds)))))))))

(event Custom|IdleAnimation
  (bind _body (Variables|Default|GetBody))
  (bind _returnvalue (Transformation|GetWorldRotation _body))
  (bind (_roll _pitch _yaw) (Math|Rotator|BreakRotator _returnvalue))
  ;[1 1 1] Animations
  (Rendering|Material|SetMaterial (Variables|Default|GetTurretBarrel) 0 "/Game/Art/Materials/TurretMaterial.TurretMaterial")
  (Variables|Default|SetCanShoot? true)
  (Timeline|PlayIdleAnimationTimeline Play
    (:Update
      (Transformation|SetWorldRotation (Variables|Default|GetBody) (Math|Rotator|MakeRotator _roll _pitch (+ _yaw (Variables|TurretTargetting|GetIdleAnimRotationSpeed))) false false))))

(event Custom|StartShooting
  (bind _timeinseconds (Variables|Default|GetTimeInSeconds))
  (bind _turretbarrel (Variables|Default|GetTurretBarrel))
  ;[1 1 1] Shoot Bullets When Target Locked
  (Components|Timeline|SetTimelineLength (Variables|Default|GetShootingTimeline) (Variables|TurretTargetting|GetTurretShootTime))
  (Timeline|ShootingTimeline PlayFromStart
    (:Update
      (if (Variables|Default|GetTargetPlayer?)
        (if (and (>= _timeinseconds (+ (Variables|Default|GetTurretRechargeTimeStart) (Variables|TurretTargetting|GetTurretRechargeTimeComplete))) (<= _timeinseconds (+ (Variables|Default|GetTurretRechargeTimeStart) (Variables|TurretTargetting|GetTurretShootTime)))) ; Change "Turret Barrel" Material To Light Up Before Firing
          (Rendering|Material|SetMaterial _turretbarrel 0 "/Game/Art/Materials/Weapons/RocketMaterial.RocketMaterial")
          (else
            (Rendering|Material|SetMaterial _turretbarrel 0 "/Game/Art/Materials/TurretMaterial.TurretMaterial")))
        (else
          (Variables|Default|SetCanShoot? true)
          (CallFunction|StopShooting))))
    (:Finished
      (Game|SpawnActorfromClass "/Game/Blueprints/EnemiesBP/EnemyWeaponsBP/TurretBulletBP.TurretBulletBP_C" (Transformation|GetWorldTransform (Variables|Default|GetBarrelOffset)) "Undefined" 0 0)
      (Variables|Default|SetTurretRechargeTimeStart (Variables|Default|GetTimeInSeconds))
      (if (Variables|Default|GetPlayerInside?)
        (Variables|Default|SetCanShoot? true)))))

(event Custom|GoToPlayerLocation
  (params (LastLocation :type Vector))
  (bind (_x _y) (Math|Vector|BreakVector LastLocation))
  (bind _returnvalue (Game|GetPlayerCharacter 0))
  (bind _returnvalue_2 (Transformation|GetActorLocation))
  (bind _returnvalue_3 (Math|Vector|MakeVector 0.0 0.0 1e+02))
  (bind _targetplayerspeed (Variables|TurretTargetting|GetTargetPlayerSpeed))
  (bind _minanglerotationindegrees (Variables|TurretTargetting|GetMinAngleRotationInDegrees))
  (bind _maxanglerotationindegrees (Variables|TurretTargetting|GetMaxAngleRotationInDegrees))
  (bind _body (Variables|Default|GetBody))
  (bind _playerinside_ (Variables|Default|GetPlayerInside?))
  (bind _body_2 (Variables|Default|GetBody))
  (bind _returnvalue_4 (Transformation|GetWorldRotation _body_2))
  (bind _rootcomponent (Variables|/Script/Engine.Actor|GetRootComponent _returnvalue))
  (bind _returnvalue_5 (Transformation|GetWorldLocation _rootcomponent))
  (bind _returnvalue_6 (- _returnvalue_5 _returnvalue_3))
  (bind _returnvalue_7 (Math|Rotator|FindLookatRotation _returnvalue_2 _returnvalue_6))
  (bind _returnvalue_8 (Class|KismetMathLibrary|RInterptoConstant _returnvalue_4 _returnvalue_7 1.0 _targetplayerspeed))
  (bind (_roll _pitch _yaw) (Math|Rotator|BreakRotator _returnvalue_8))
  (bind _returnvalue_9 (Math|Float|ClampAngle _pitch _minanglerotationindegrees _maxanglerotationindegrees))
  (bind _returnvalue_10 (Math|Rotator|MakeRotator _roll _returnvalue_9 _yaw))
  ;[1 1 1] Go To Player When Turret Loses Sight Of Player
  (Variables|Default|SetFlyingEnabled? true)
  (Variables|Default|SetNewLocation (Math|Vector|MakeVector (- _x (Math|Random|RandomFloatinRange -2e+02 2e+02)) (- _y (Math|Random|RandomFloatinRange -2e+02 2e+02)) (.Z (Math|Vector|BreakVector (Transformation|GetActorLocation)))))
  (Timeline|TryToTrackPlayer PlayFromStart
    (:Update
      (if (Class|AIBlueprintHelperLibrary|IsValidAIRotation _returnvalue_10)
        (Utilities|IsValid _body
          (:Is%20Valid
            (Transformation|SetWorldRotation _body _returnvalue_10 false false)))))
    (:Finished
      (if (Variables|Default|GetTargetPlayer?)
        (if _playerinside_
          (CallFunction|ToTargetPlayerTimeline)
          (else
            (CallFunction|IdleAnimation :!label _label)))
        (elif _playerinside_
          (goto _label)
          (else
            (goto _label)))))))

(event Custom|ToTargetPlayerTimeline
  (bind _body (Variables|Default|GetBody))
  ;[1 1 1] Targetting Player
  (Timeline|TargetPlayer Play
    (:Update
      (if (and (Utilities|IsValid _body) (Class|AIBlueprintHelperLibrary|IsValidAIRotation (Math|Rotator|MakeRotator (.Roll (Math|Rotator|BreakRotator (Class|KismetMathLibrary|RInterptoConstant (Transformation|GetWorldRotation (Variables|Default|GetBody)) (Math|Rotator|FindLookatRotation (Transformation|GetActorLocation) (- (Transformation|GetWorldLocation (Variables|/Game/Blueprints/PlayerBP/FPSController.FPSController_C|GetRootLocation (stale OnComponentBeginOverlap(Trigger) _asfpscontroller))) (Math|Vector|MakeVector 0.0 0.0 1e+02))) 1.0 (Variables|TurretTargetting|GetTargetPlayerSpeed)))) (Math|Float|ClampAngle (.Pitch (Math|Rotator|BreakRotator (Class|KismetMathLibrary|RInterptoConstant (Transformation|GetWorldRotation (Variables|Default|GetBody)) (Math|Rotator|FindLookatRotation (Transformation|GetActorLocation) (- (Transformation|GetWorldLocation (Variables|/Game/Blueprints/PlayerBP/FPSController.FPSController_C|GetRootLocation (stale OnComponentBeginOverlap(Trigger) _asfpscontroller))) (Math|Vector|MakeVector 0.0 0.0 1e+02))) 1.0 (Variables|TurretTargetting|GetTargetPlayerSpeed)))) (Variables|TurretTargetting|GetMinAngleRotationInDegrees) (Variables|TurretTargetting|GetMaxAngleRotationInDegrees)) (.Yaw (Math|Rotator|BreakRotator (Class|KismetMathLibrary|RInterptoConstant (Transformation|GetWorldRotation (Variables|Default|GetBody)) (Math|Rotator|FindLookatRotation (Transformation|GetActorLocation) (- (Transformation|GetWorldLocation (Variables|/Game/Blueprints/PlayerBP/FPSController.FPSController_C|GetRootLocation (stale OnComponentBeginOverlap(Trigger) _asfpscontroller))) (Math|Vector|MakeVector 0.0 0.0 1e+02))) 1.0 (Variables|TurretTargetting|GetTargetPlayerSpeed)))))))
        (Transformation|SetWorldRotation _body (Math|Rotator|MakeRotator (.Roll (Math|Rotator|BreakRotator (Class|KismetMathLibrary|RInterptoConstant (Transformation|GetWorldRotation (Variables|Default|GetBody)) (Math|Rotator|FindLookatRotation (Transformation|GetActorLocation) (- (Transformation|GetWorldLocation (Variables|/Game/Blueprints/PlayerBP/FPSController.FPSController_C|GetRootLocation (stale OnComponentBeginOverlap(Trigger) _asfpscontroller))) (Math|Vector|MakeVector 0.0 0.0 1e+02))) 1.0 (Variables|TurretTargetting|GetTargetPlayerSpeed)))) (Math|Float|ClampAngle (.Pitch (Math|Rotator|BreakRotator (Class|KismetMathLibrary|RInterptoConstant (Transformation|GetWorldRotation (Variables|Default|GetBody)) (Math|Rotator|FindLookatRotation (Transformation|GetActorLocation) (- (Transformation|GetWorldLocation (Variables|/Game/Blueprints/PlayerBP/FPSController.FPSController_C|GetRootLocation (stale OnComponentBeginOverlap(Trigger) _asfpscontroller))) (Math|Vector|MakeVector 0.0 0.0 1e+02))) 1.0 (Variables|TurretTargetting|GetTargetPlayerSpeed)))) (Variables|TurretTargetting|GetMinAngleRotationInDegrees) (Variables|TurretTargetting|GetMaxAngleRotationInDegrees)) (.Yaw (Math|Rotator|BreakRotator (Class|KismetMathLibrary|RInterptoConstant (Transformation|GetWorldRotation (Variables|Default|GetBody)) (Math|Rotator|FindLookatRotation (Transformation|GetActorLocation) (- (Transformation|GetWorldLocation (Variables|/Game/Blueprints/PlayerBP/FPSController.FPSController_C|GetRootLocation (stale OnComponentBeginOverlap(Trigger) _asfpscontroller))) (Math|Vector|MakeVector 0.0 0.0 1e+02))) 1.0 (Variables|TurretTargetting|GetTargetPlayerSpeed))))) false false)
        (Utilities|LineTrace
          (:End
            (if (and (Variables|Default|GetCanShoot?) (Variables|Default|GetTargetPlayer?))
              (Variables|Default|SetCanShoot? false)
              (CallFunction|StartShooting)
              (Variables|Default|SetTurretRechargeTimeStart (Variables|Default|GetTimeInSeconds)))))))))

(event Custom|StopIdleAnimation
  (bind _body (Variables|Default|GetBody))
  (bind _returnvalue (Transformation|GetWorldRotation _body))
  (bind (_roll _pitch _yaw) (Math|Rotator|BreakRotator _returnvalue))
  ;[1 1 1] Animations
  (Timeline|PlayIdleAnimationTimeline Stop
    (:Update
      (Transformation|SetWorldRotation (Variables|Default|GetBody) (Math|Rotator|MakeRotator _roll _pitch (+ _yaw (Variables|TurretTargetting|GetIdleAnimRotationSpeed))) false false))))

(event Custom|AreaSweep
  (bind _sweepareafactor (Variables|TurretTargetting|GetSweepAreaFactor))
  (bind _initialturretlocation (Variables|Default|GetInitialTurretLocation))
  (bind (_x _y) (Math|Vector|BreakVector _initialturretlocation))
  ;[1 1 1] Flying Mechanics
  (if (Variables|Default|GetFlyingEnabled?)
    (Variables|Default|SetNewLocation (Math|Vector|MakeVector (Math|Random|RandomFloatinRange (- _x _sweepareafactor) (+ _x _sweepareafactor)) (Math|Random|RandomFloatinRange (- _y _sweepareafactor) (+ _y _sweepareafactor)) (.Z (Math|Vector|BreakVector (Transformation|GetActorLocation)))))
    (CallFunction|StartSweep)))

(event Custom|StartSweep
  ;[1 1 1] Flying Mechanics
  (Timeline|FlyingMechanicsTimeline Play
    (:Update
      (Transformation|SetActorLocation (Math|Interpolation|VInterptoConstant (Transformation|GetActorLocation) (Variables|Default|GetNewLocation) 1.0 1e+01) false false))))

(event Custom|StartTargetting
  ;[1 1 1] Flying Mechanics
  (Timeline|FlyingMechanicsTimeline Stop
    (:Update
      (Transformation|SetActorLocation (Math|Interpolation|VInterptoConstant (Transformation|GetActorLocation) (Variables|Default|GetNewLocation) 1.0 1e+01) false false))))

(event Custom|StartLineTrace
  ;[1 1 1] Targetting Player
  (Utilities|LineTrace
    (:End
      (if (and (Variables|Default|GetCanShoot?) (Variables|Default|GetTargetPlayer?))
        (Variables|Default|SetCanShoot? false)
        (CallFunction|StartShooting)
        (Variables|Default|SetTurretRechargeTimeStart (Variables|Default|GetTimeInSeconds))))))

(event Custom|StopShooting
  (bind _timeinseconds (Variables|Default|GetTimeInSeconds))
  (bind _turretbarrel (Variables|Default|GetTurretBarrel))
  ;[1 1 1] Shoot Bullets When Target Locked
  (Timeline|ShootingTimeline Stop
    (:Update
      (if (Variables|Default|GetTargetPlayer?)
        (if (and (>= _timeinseconds (+ (Variables|Default|GetTurretRechargeTimeStart) (Variables|TurretTargetting|GetTurretRechargeTimeComplete))) (<= _timeinseconds (+ (Variables|Default|GetTurretRechargeTimeStart) (Variables|TurretTargetting|GetTurretShootTime)))) ; Change "Turret Barrel" Material To Light Up Before Firing
          (Rendering|Material|SetMaterial _turretbarrel 0 "/Game/Art/Materials/Weapons/RocketMaterial.RocketMaterial")
          (else
            (Rendering|Material|SetMaterial _turretbarrel 0 "/Game/Art/Materials/TurretMaterial.TurretMaterial")))
        (else
          (Variables|Default|SetCanShoot? true)
          (CallFunction|StopShooting))))
    (:Finished
      (Game|SpawnActorfromClass "/Game/Blueprints/EnemiesBP/EnemyWeaponsBP/TurretBulletBP.TurretBulletBP_C" (Transformation|GetWorldTransform (Variables|Default|GetBarrelOffset)) "Undefined" 0 0)
      (Variables|Default|SetTurretRechargeTimeStart (Variables|Default|GetTimeInSeconds))
      (if (Variables|Default|GetPlayerInside?)
        (Variables|Default|SetCanShoot? true)))))

(event EventTick
  (params (DeltaSeconds :type Float%20%28single-precision%29))
  ;[1 1 1] Setting DeltaTime And TimeInSeconds
  (bind _output_get (Variables|Default|SetDeltaTime DeltaSeconds))
  (Variables|Default|SetTimeInSeconds (+ _output_get (Variables|Default|GetTimeInSeconds))))

(event Game|Damage|EventAnyDamage
  (params (Damage :type Float%20%28single-precision%29) (DamageType :type Damage%20Type%20Object%20Reference) (InstigatedBy :type Controller%20Object%20Reference) (DamageCauser :type Actor%20Object%20Reference))
  ;[0 1 0.05932] Health System
  (bind _output_get (Variables|Default|SetCurrentHealth (- (Variables|Default|GetCurrentHealth) Damage)))
  (if (<= _output_get 0.0)
    (Actor|DestroyActor)))

(event EventBeginPlay
  (bind _body (Variables|Default|GetBody))
  (bind _returnvalue (Transformation|GetWorldRotation _body))
  (bind (_roll _pitch _yaw) (Math|Rotator|BreakRotator _returnvalue))
  ;[1 1 1] Animations
  (Utilities|BeginPlayReferences)
  (Variables|Default|SetInitialTurretLocation (Transformation|GetActorLocation))
  (Utilities|Time|SetTimerbyFunctionName 0 "AreaSweep" 5.0 true)
  (Timeline|PlayIdleAnimationTimeline Play
    (:Update
      (Transformation|SetWorldRotation (Variables|Default|GetBody) (Math|Rotator|MakeRotator _roll _pitch (+ _yaw (Variables|TurretTargetting|GetIdleAnimRotationSpeed))) false false))))

(fn ConstructionScript
  (bind _spotlight (Variables|Default|GetSpotLight))
  (bind _barreloffset (Variables|Default|GetBarrelOffset))
  (bind _trigger (Variables|Default|GetTrigger))
  (Components|Capsule|SetCapsuleHalfHeight _trigger (Variables|TriggerCapsuleProperties|GetTriggerSize) false)
  (Components|Capsule|SetCapsuleRadius _trigger (Variables|TurretTargetting|GetTriggerRadius) true)
  (Transformation|SetWorldLocation _trigger (+ (* (Math|Vector|GetForwardVector _barreloffset) (Variables|TriggerCapsuleProperties|GetChangeTriggerLocalOffset)) (Transformation|GetWorldLocation _barreloffset)) false false)
  (Transformation|SetWorldScale3D (Variables|Default|GetViewcone) (Variables|ViewCone|GetViewConeScale))
  (Rendering|Components|Light|SetIntensity _spotlight (Variables|SpotLightProperties|GetSpotLightIntensity))
  (Rendering|Components|Light|SetLightColor _spotlight (Variables|SpotLightProperties|GetSpotLightColor) true)
  (Rendering|Lighting|SetOuterConeAngle _spotlight (Variables|SpotLightProperties|GetOuterConeAngle)))