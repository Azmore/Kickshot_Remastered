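; Soldier enemy NPC that tracks its health, displays it on a floating health bar and is destroyed when health runs out.
; BeginPlay caches the player's FPSController and fills the EnemyHealth widget from MaxHealth.
; AnyDamage lowers health, updates the widget and briefly shows the bar through a Delay.
; Tick rotates the bar component toward the player using a look-at from the soldier's location.
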(event Custom|HealthBarVisibility
  (bind _healthbar (Variables|Default|GetHealthBar))
  ;[1 1 1] Set Health Bar Visibility
  (Rendering|SetVisibility _healthbar true false)
  (Utilities|FlowControl|Delay 5.0)
  (Rendering|SetVisibility _healthbar false false))

(event EventTick
  (params (DeltaSeconds :type Float%20%28single-precision%29))
  (bind _fpscontrollerreference (Variables|Default|GetFPSControllerReference))
  ;[1 1 1] Widget Face The Player
  (Utilities|IsValid _fpscontrollerreference
    (:Is%20Valid
      (Transformation|SetWorldRotation (Variables|Default|GetHealthBar) (Math|Rotator|FindLookatRotation (Transformation|GetActorLocation) (Transformation|GetActorLocation _fpscontrollerreference)) false false))))

(event Game|Damage|EventAnyDamage
  (params (Damage :type Float%20%28single-precision%29) (DamageType :type Damage%20Type%20Object%20Reference) (InstigatedBy :type Controller%20Object%20Reference) (DamageCauser :type Actor%20Object%20Reference))
  ;[0 1 0.05932] Health System
  (CallFunction|HealthBarVisibility)
  (bind _asenemy_health (Utilities|Casting|CastToEnemyHealth (UserInterface|GetUserWidgetObject (Variables|Default|GetHealthBar))))
  (bind _output_get (Variables|Default|SetCurrentHealth (- (Variables|Default|GetCurrentHealth) Damage)))
  (bind _output_get_2 (Variables|/Game/Widgets/EnemyHealth.EnemyHealth_C|SetCurrentHealth _asenemy_health _output_get))
  (if (<= _output_get_2 0.0)
    (Actor|DestroyActor)))

(event EventBeginPlay
  (bind _asfpscontroller (Utilities|Casting|CastToFPSController (Game|GetPlayerCharacter 0)))
  (Variables|Default|SetFPSControllerReference _asfpscontroller)
  ;[0 1 0.05932] Health System
  (bind _asenemy_health (Utilities|Casting|CastToEnemyHealth (UserInterface|GetUserWidgetObject (Variables|Default|GetHealthBar))))
  (bind _output_get (Variables|Default|SetCurrentHealth (Variables|Default|GetMaxHealth)))
  (Variables|/Game/Widgets/EnemyHealth.EnemyHealth_C|SetCurrentHealth _asenemy_health _output_get))

(fn ConstructionScript)