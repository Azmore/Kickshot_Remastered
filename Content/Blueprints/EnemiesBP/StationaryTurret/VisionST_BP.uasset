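; Stationary turret enemy that tracks and shoots the player, and is destroyed when its health runs out.
; Trigger overlap stops the idle spin and starts a timeline that turns the body toward the player with clamped pitch.
; A barrel line trace for the "Player" tag gates a looping shooting timeline, which swaps barrel material before spawning each TurretBulletBP.
; Leaving the trigger levels the body and resumes spinning.
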(event OnComponentBeginOverlap(Trigger)
  (params (OverlappedComponent :type Primitive%20Component%20Object%20Reference) (OtherActor :type Actor%20Object%20Reference) (OtherComp :type Primitive%20Component%20Object%20Reference) (OtherBodyIndex :type Integer) (bFromSweep :type Boolean) (SweepResult :type Hit%20Result%20Structure%20%28by%20ref%29))
  ;[1 1 1] Targetting Player
  (bind _asfpscontroller (Utilities|Casting|CastToFPSController OtherActor))
  (CallFunction|StopIdleAnimation)
  (Timeline|TargetPlayer PlayFromStart
    (:Update
      (Transformation|SetWorldRotation (Variables|Default|GetBody) (Math|Rotator|MakeRotator (.Roll (Math|Rotator|BreakRotator (Class|KismetMathLibrary|RInterptoConstant (Transformation|GetWorldRotation (Variables|Default|GetBody)) (Math|Rotator|FindLookatRotation (Transformation|GetActorLocation) (- (Transformation|GetWorldLocation (Variables|/Game/Blueprints/PlayerBP/FPSController.FPSController_C|GetRootLocation _asfpscontroller)) (Math|Vector|MakeVector 0.0 0.0 1e+02))) 1.0 (Variables|Default|GetTargetPlayerSpeed)))) (Math|Float|ClampAngle (.Pitch (Math|Rotator|BreakRotator (Class|KismetMathLibrary|RInterptoConstant (Transformation|GetWorldRotation (Variables|Default|GetBody)) (Math|Rotator|FindLookatRotation (Transformation|GetActorLocation) (- (Transformation|GetWorldLocation (Variables|/Game/Blueprints/PlayerBP/FPSController.FPSController_C|GetRootLocation _asfpscontroller)) (Math|Vector|MakeVector 0.0 0.0 1e+02))) 1.0 (Variables|Default|GetTargetPlayerSpeed)))) (Variables|Default|GetMinAngleRotationInDegrees) (Variables|Default|GetMaxAngleRotationInDegrees)) (.Yaw (Math|Rotator|BreakRotator (Class|KismetMathLibrary|RInterptoConstant (Transformation|GetWorldRotation (Variables|Default|GetBody)) (Math|Rotator|FindLookatRotation (Transformation|GetActorLocation) (- (Transformation|GetWorldLocation (Variables|/Game/Blueprints/PlayerBP/FPSController.FPSController_C|GetRootLocation _asfpscontroller)) (Math|Vector|MakeVector 0.0 0.0 1e+02))) 1.0 (Variables|Default|GetTargetPlayerSpeed))))) false false)
      (Utilities|LineTrace
        (:End
          (if (and (Variables|Default|GetCanShoot?) (Variables|Default|GetTargetPlayer?))
            (Variables|Default|SetCanShoot? false)
            (CallFunction|StartShooting)
            (Variables|Default|SetCustomTime1 (Variables|Default|GetTimeInSeconds))))))))

(event OnComponentEndOverlap(Trigger)
  (params (OverlappedComponent :type Primitive%20Component%20Object%20Reference) (OtherActor :type Actor%20Object%20Reference) (OtherComp :type Primitive%20Component%20Object%20Reference) (OtherBodyIndex :type Integer))
  ;[1 1 1] Targetting Player
  (Utilities|Casting|CastToFPSController OtherActor)
  (Variables|Default|SetTargetPlayer? false)
  (CallFunction|IdleAnimation)
  (Timeline|TargetPlayer Stop
    (:Update
      (Transformation|SetWorldRotation (Variables|Default|GetBody) (Math|Rotator|MakeRotator (.Roll (Math|Rotator|BreakRotator (Class|KismetMathLibrary|RInterptoConstant (Transformation|GetWorldRotation (Variables|Default|GetBody)) (Math|Rotator|FindLookatRotation (Transformation|GetActorLocation) (- (Transformation|GetWorldLocation (Variables|/Game/Blueprints/PlayerBP/FPSController.FPSController_C|GetRootLocation (stale OnComponentBeginOverlap(Trigger) _asfpscontroller))) (Math|Vector|MakeVector 0.0 0.0 1e+02))) 1.0 (Variables|Default|GetTargetPlayerSpeed)))) (Math|Float|ClampAngle (.Pitch (Math|Rotator|BreakRotator (Class|KismetMathLibrary|RInterptoConstant (Transformation|GetWorldRotation (Variables|Default|GetBody)) (Math|Rotator|FindLookatRotation (Transformation|GetActorLocation) (- (Transformation|GetWorldLocation (Variables|/Game/Blueprints/PlayerBP/FPSController.FPSController_C|GetRootLocation (stale OnComponentBeginOverlap(Trigger) _asfpscontroller))) (Math|Vector|MakeVector 0.0 0.0 1e+02))) 1.0 (Variables|Default|GetTargetPlayerSpeed)))) (Variables|Default|GetMinAngleRotationInDegrees) (Variables|Default|GetMaxAngleRotationInDegrees)) (.Yaw (Math|Rotator|BreakRotator (Class|KismetMathLibrary|RInterptoConstant (Transformation|GetWorldRotation (Variables|Default|GetBody)) (Math|Rotator|FindLookatRotation (Transformation|GetActorLocation) (- (Transformation|GetWorldLocation (Variables|/Game/Blueprints/PlayerBP/FPSController.FPSController_C|GetRootLocation (stale OnComponentBeginOverlap(Trigger) _asfpscontroller))) (Math|Vector|MakeVector 0.0 0.0 1e+02))) 1.0 (Variables|Default|GetTargetPlayerSpeed))))) false false)
      (Utilities|LineTrace
        (:End
          (if (and (Variables|Default|GetCanShoot?) (Variables|Default|GetTargetPlayer?))
            (Variables|Default|SetCanShoot? false)
            (CallFunction|StartShooting)
            (Variables|Default|SetCustomTime1 (Variables|Default|GetTimeInSeconds))))))))

(event Custom|IdleAnimation
  (bind _body (Variables|Default|GetBody))
  (bind _timeinseconds (Variables|Default|GetTimeInSeconds))
  (bind _turretbarrel (Variables|Default|GetTurretBarrel))
  (bind _body_2 (Variables|Default|GetBody))
  (bind _returnvalue (Transformation|GetWorldRotation _body_2))
  (bind _returnvalue_2 (Transformation|GetWorldRotation _body))
  (bind (_roll _pitch _yaw) (Math|Rotator|BreakRotator _returnvalue))
  (bind (_roll_2 _pitch_2 _yaw_2) (Math|Rotator|BreakRotator _returnvalue_2))
  (bind _returnvalue_3 (Math|Rotator|MakeRotator _roll_2 0.0 _yaw_2))
  (bind _returnvalue_4 (Class|KismetMathLibrary|RInterptoConstant _returnvalue_2 _returnvalue_3 1.0 1.0))
  (bind (_roll_3 _pitch_3 _yaw_3) (Math|Rotator|BreakRotator _returnvalue_4))
  ;[1 1 1] Animations
  (Rendering|Material|SetMaterial (Variables|Default|GetTurretBarrel) 0 "/Game/Art/Materials/TurretMaterial.TurretMaterial")
  (Variables|Default|SetCanShoot? true)
  (Timeline|TurretStraightTimeline PlayFromStart
    (:Update
      (Transformation|SetWorldRotation (Variables|Default|GetBody) (Math|Rotator|MakeRotator _roll_3 _pitch_3 (+ _yaw_3 (Variables|Default|GetIdleAnimRotationSpeed))) false false)
      ;[1 1 1] Shoot Bullets When Target Locked
      (Timeline|ShootingTimeline Stop
        (:Update
          (if (Variables|Default|GetTargetPlayer?)
            (if (and (>= _timeinseconds (+ (Variables|Default|GetCustomTime1) (Variables|Default|GetTurretRechargeTime))) (<= _timeinseconds (+ (Variables|Default|GetCustomTime1) (Variables|Default|GetTurretShootTime))))
              (Rendering|Material|SetMaterial _turretbarrel 0 "/Game/Art/Materials/Weapons/RocketMaterial.RocketMaterial")
              (else
                (Rendering|Material|SetMaterial _turretbarrel 0 "/Game/Art/Materials/TurretMaterial.TurretMaterial")))
            (else
              (Variables|Default|SetCanShoot? true)
              (Timeline|ShootingTimeline Stop))))
        (:Finished
          (Game|SpawnActorfromClass "/Game/Blueprints/EnemiesBP/EnemyWeaponsBP/TurretBulletBP.TurretBulletBP_C" (Transformation|GetWorldTransform (Variables|Default|GetBarrelOffset)) "Undefined" 0 0)
          (Variables|Default|SetCustomTime1 (Variables|Default|GetTimeInSeconds))
          (Timeline|ShootingTimeline PlayFromStart))))
    (:Finished
      (Timeline|PlayIdleAnimationTimeline Play
        (:Update
          (Transformation|SetWorldRotation (Variables|Default|GetBody) (Math|Rotator|MakeRotator _roll _pitch (+ _yaw (Variables|Default|GetIdleAnimRotationSpeed))) false false))))))

(event Custom|StartShooting
  (bind _timeinseconds (Variables|Default|GetTimeInSeconds))
  (bind _turretbarrel (Variables|Default|GetTurretBarrel))
  ;[1 1 1] Shoot Bullets When Target Locked
  (Components|Timeline|SetTimelineLength (Variables|Default|GetShootingTimeline) (Variables|Default|GetTurretShootTime))
  (Timeline|ShootingTimeline PlayFromStart
    (:Update
      (if (Variables|Default|GetTargetPlayer?)
        (if (and (>= _timeinseconds (+ (Variables|Default|GetCustomTime1) (Variables|Default|GetTurretRechargeTime))) (<= _timeinseconds (+ (Variables|Default|GetCustomTime1) (Variables|Default|GetTurretShootTime))))
          (Rendering|Material|SetMaterial _turretbarrel 0 "/Game/Art/Materials/Weapons/RocketMaterial.RocketMaterial")
          (else
            (Rendering|Material|SetMaterial _turretbarrel 0 "/Game/Art/Materials/TurretMaterial.TurretMaterial")))
        (else
          (Variables|Default|SetCanShoot? true)
          (Timeline|ShootingTimeline Stop))))
    (:Finished
      (Game|SpawnActorfromClass "/Game/Blueprints/EnemiesBP/EnemyWeaponsBP/TurretBulletBP.TurretBulletBP_C" (Transformation|GetWorldTransform (Variables|Default|GetBarrelOffset)) "Undefined" 0 0)
      (Variables|Default|SetCustomTime1 (Variables|Default|GetTimeInSeconds))
      (Timeline|ShootingTimeline PlayFromStart))))

(event Custom|StopIdleAnimation
  (bind _body (Variables|Default|GetBody))
  (bind _returnvalue (Transformation|GetWorldRotation _body))
  (bind (_roll _pitch _yaw) (Math|Rotator|BreakRotator _returnvalue))
  ;[1 1 1] Animations
  (Timeline|PlayIdleAnimationTimeline Stop
    (:Update
      (Transformation|SetWorldRotation (Variables|Default|GetBody) (Math|Rotator|MakeRotator _roll _pitch (+ _yaw (Variables|Default|GetIdleAnimRotationSpeed))) false false))))

(event EventTick
  (params (DeltaSeconds :type Float%20%28single-precision%29))
  ;[1 1 1] Setting DeltaTime And TimeInSeconds
  (bind _output_get (Variables|Default|SetDeltaTime DeltaSeconds))
  (Variables|Default|SetTimeInSeconds (+ _output_get (Variables|Default|GetTimeInSeconds))))

(event Game|Damage|EventAnyDamage
  (params (Damage :type Float%20%28single-precision%29) (DamageType :type Damage%20Type%20Object%20Reference) (InstigatedBy :type Controller%20Object%20Reference) (DamageCauser :type Actor%20Object%20Reference))
  ;[0 1 0.05932] Health System
  (bind _output_get (Variables|Default|SetTurretHealth (- (Variables|Default|GetTurretHealth) Damage)))
  (Development|PrintString (Utilities|String|Append "Turret Health : " (Utilities|String|ToString(Float) _output_get)) true true "(R=0.000000,G=1.000000,B=0.059316,A=1.000000)" 3.0)
  (if (<= _output_get 0.0)
    (Actor|DestroyActor)))

(event EventBeginPlay
  (bind _body (Variables|Default|GetBody))
  (bind _returnvalue (Transformation|GetWorldRotation _body))
  (bind (_roll _pitch _yaw) (Math|Rotator|BreakRotator _returnvalue))
  ;[1 1 1] Animations
  (Timeline|PlayIdleAnimationTimeline Play
    (:Update
      (Transformation|SetWorldRotation (Variables|Default|GetBody) (Math|Rotator|MakeRotator _roll _pitch (+ _yaw (Variables|Default|GetIdleAnimRotationSpeed))) false false))))

(fn ConstructionScript)